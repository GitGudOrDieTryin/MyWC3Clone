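; RTS player controller that drives the RTSCamera_BP pawn with a visible cursor and Game-and-UI input.
; Axis input moves the pawn relative to its facing via a macro with a speed modifier, pinning height on one axis; zoom clamps spring arm length.
; Holding CameraPan disables axis movement and opens gates for mouse yaw and clamped pitch.
; A macro converts screen-edge cursor position into local-offset scrolling; EdgeScroll and EdgeScrollTol functions are unfinished stubs.
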(event EventBeginPlay
  (bind _asrtscamera_bp (Utilities|Casting|CastToRTSCamera_BP (Pawn|GetControlledPawn)))
  (Variables|Default|SetCameraPawnReference_C _asrtscamera_bp)
  (Input|SetInputModeGameandUI self 0 "DoNotLock" true)
  (Variables|Default|SetbShowMouseCursor true))

(event EventTick
  (params (DeltaSeconds :type Float%20%28single-precision%29))
  ;[1 1 1] Pan Controls
)

(event Input|ActionEvents|InputActionZoomReset
  (params (Key :type Key%20Structure :default "None"))
  ;[1 1 1] Reset Zoom
  (:Pressed
    (Variables|/Script/Engine.SpringArmComponent|SetTargetArmLength (Variables|/Game/Blueprints/RTSCamera_BP.RTSCamera_BP_C|GetSpringArm (Variables|Default|GetCameraPawnReference_C)) 1.5e+03)))

(event Input|ActionEvents|InputActionZoomIn
  (params (Key :type Key%20Structure :default "None"))
  (bind _camerapawnreference_c (Variables|Default|GetCameraPawnReference_C))
  (bind _springarm (Variables|/Game/Blueprints/RTSCamera_BP.RTSCamera_BP_C|GetSpringArm _camerapawnreference_c))
  ;[1 1 1] Zoom in and Out with a maximum and minimum zoom limit
  (:Pressed
    (Variables|/Script/Engine.SpringArmComponent|SetTargetArmLength _springarm (Math|Float|Clamp(Float) (- (Variables|/Script/Engine.SpringArmComponent|GetTargetArmLength _springarm) (Variables|Default|GetZoomSpeed)) (Variables|Default|GetMinZoomLimit) (Variables|Default|GetMaxZoomLimit)))))

(event Input|ActionEvents|InputActionZoomOut
  (params (Key :type Key%20Structure :default "None"))
  (bind _camerapawnreference_c (Variables|Default|GetCameraPawnReference_C))
  (bind _springarm (Variables|/Game/Blueprints/RTSCamera_BP.RTSCamera_BP_C|GetSpringArm _camerapawnreference_c))
  ;[1 1 1] Zoom in and Out with a maximum and minimum zoom limit
  (:Pressed
    (Variables|/Script/Engine.SpringArmComponent|SetTargetArmLength _springarm (Math|Float|Clamp(Float) (+ (Variables|/Script/Engine.SpringArmComponent|GetTargetArmLength _springarm) (Variables|Default|GetZoomSpeed)) (Variables|Default|GetMinZoomLimit) (Variables|Default|GetMaxZoomLimit)))))

(event Input|ActionEvents|InputActionPanReset
  (params (Key :type Key%20Structure :default "None"))
  (bind _camerapawnreference_c (Variables|Default|GetCameraPawnReference_C))
  ;[1 1 1] Pan Controls
  ;;[1 1 1] Reset Pan
  (:Pressed
    (Transformation|SetActorRotation _camerapawnreference_c (Math|Rotator|MakeRotator (.Roll (Math|Rotator|BreakRotator (Transformation|GetActorRotation _camerapawnreference_c))) 0.0 0.0))))

(event Input|ActionEvents|InputActionCameraPan
  (params (Key :type Key%20Structure :default "None"))
  (bind _camerapawnreference_c (Variables|Default|GetCameraPawnReference_C))
  (bind _returnvalue (Transformation|GetActorRotation _camerapawnreference_c))
  (bind (_roll _pitch _yaw) (Math|Rotator|BreakRotator _returnvalue))
  ;[1 1 1] Pan Controls
  ;;[1 1 1] Pan Pitch(Y Axis)
  (:Pressed
    (Variables|Default|SetDisableCamMovement true)
    (Utilities|FlowControl|Gate true) ; enters at Open
  )
  (:Released
    (Variables|Default|SetDisableCamMovement false)
    (Utilities|FlowControl|Gate true) ; enters at Close
  ))

(event Input|ActionEvents|InputActionCameraPan
  (params (Key :type Key%20Structure :default "None"))
  (bind _camerapawnreference_c (Variables|Default|GetCameraPawnReference_C))
  (bind _returnvalue (Transformation|GetActorRotation _camerapawnreference_c))
  (bind (_roll _pitch _yaw) (Math|Rotator|BreakRotator _returnvalue))
  ;[1 1 1] Pan Controls
  ;;[1 1 1] Pan Yaw(X Axis)
  (:Pressed
    (Variables|Default|SetDisableCamMovement true)
    (Utilities|FlowControl|Gate true) ; enters at Open
  )
  (:Released
    (Variables|Default|SetDisableCamMovement false)
    (Utilities|FlowControl|Gate true) ; enters at Close
  ))

(event Input|ActionEvents|InputActionCameraSpeedModifier
  (params (Key :type Key%20Structure :default "None"))
  ;[1 1 1] Movement Speed Modifier with shift
  (:Pressed
    (Variables|Default|SetMovementSpeedModifier 1.75))
  (:Released
    (Variables|Default|SetMovementSpeedModifier 1.0)))

(event Input|AxisEvents|InputAxisMouseX
  (params (AxisValue :type Float%20%28single-precision%29))
  ;[1 1 1] Edge Scroll Functionality
  (bind (_deltaspeedx _deltaspeedy) (Utilities|EdgeScrollMacro))
  (Transformation|AddActorLocalOffset (Variables|Default|GetCameraPawnReference_C) (Math|Vector|MakeVector _deltaspeedx _deltaspeedy 0.0) true false))

(event Input|AxisEvents|InputAxisMouseY
  (params (AxisValue :type Float%20%28single-precision%29))
  ;[1 1 1] Edge Scroll Functionality
  (Utilities|EdgeScrollMacro) ; enters at MouseY
)

(event Input|AxisEvents|InputAxisMoveforward
  (params (AxisValue :type Float%20%28single-precision%29))
  ;[1 1 1] Movement Controls - Macro used for networking and readability purposes
  (if (not (Variables|Default|GetDisableCamMovement))
    (Utilities|BasicMovementControll (stale Input|AxisEvents|InputAxisMoveRight AxisValue) AxisValue)))

(event Input|AxisEvents|InputAxisMoveRight
  (params (AxisValue :type Float%20%28single-precision%29))
  ;[1 1 1] Movement Controls - Macro used for networking and readability purposes
  (if (not (Variables|Default|GetDisableCamMovement))
    (Utilities|BasicMovementControll AxisValue (stale Input|AxisEvents|InputAxisMoveforward AxisValue)) ; enters at Move Right
  ))

(event Input|MouseEvents|MouseX
  (params (AxisValue :type Float%20%28single-precision%29))
  (bind _camerapawnreference_c (Variables|Default|GetCameraPawnReference_C))
  (bind _returnvalue (Transformation|GetActorRotation _camerapawnreference_c))
  (bind (_roll _pitch _yaw) (Math|Rotator|BreakRotator _returnvalue))
  ;[1 1 1] Pan Controls
  ;;[1 1 1] Pan Yaw(X Axis)
  (Utilities|FlowControl|Gate true
    (:Exit
      (Transformation|SetActorRotation _camerapawnreference_c (Math|Rotator|MakeRotator _roll _pitch (+ _yaw (* AxisValue (Variables|Default|GetPanSpeed))))))))

(event Input|MouseEvents|MouseY
  (params (AxisValue :type Float%20%28single-precision%29))
  (bind _camerapawnreference_c (Variables|Default|GetCameraPawnReference_C))
  (bind _returnvalue (Transformation|GetActorRotation _camerapawnreference_c))
  (bind (_roll _pitch _yaw) (Math|Rotator|BreakRotator _returnvalue))
  ;[1 1 1] Pan Controls
  ;;[1 1 1] Pan Pitch(Y Axis)
  (Utilities|FlowControl|Gate true
    (:Exit
      (Transformation|SetActorRotation _camerapawnreference_c (Math|Rotator|MakeRotator _roll (Math|Float|Clamp(Float) (+ _pitch (* AxisValue (Variables|Default|GetPanSpeed))) -25.0 45.0) _yaw)))))

(fn ConstructionScript)

(fn EdgeScrollTol)

(fn EdgeScroll
  (params (NewParam :type Vector%202D%20Structure) (NewParam1 :type Vector%202D%20Structure)))