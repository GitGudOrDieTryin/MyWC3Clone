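; RTS player controller Blueprint with helper functions for swipe-drag and screen-edge scrolling; its event graph is empty.
; Swipe functions trace under the cursor, store start and end world points, and return a flattened start-minus-current delta during updates.
; IsScrolling is unfinished: it tests left and right screen margins, then unconditionally overwrites the result with MouseDown, leaves the vertical check unused and never reaches its return.
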(event EventBeginPlay)

(event EventTick
  (params (DeltaSeconds :type Float%20%28single-precision%29)))

(fn ConstructionScript)

(fn OnSwipeStarted
  (Variables|Default|SetStartSwipeCoords%20	 (.Location (Collision|BreakHitResult (.HitResult (Game|Player|GetHitResultUnderCursorbyChannel "TraceTypeQuery1" true))))))

(fn OnSwipeEnded
  (Variables|Default|SetEndSwipeCoords%20	 (.Location (Collision|BreakHitResult (.HitResult (Game|Player|GetHitResultUnderCursorbyChannel "TraceTypeQuery1" true)))))
  (Variables|Default|SetStartSwipeCoords%20	 "0, 0, 0"))

(fn OnSwipeUpdate
  (LocalVariables|SetLocalNewSwipeCoords (.Location (Collision|BreakHitResult (.HitResult (Game|Player|GetHitResultUnderCursorbyChannel "TraceTypeQuery1" true)))))
  (bind _output_get (LocalVariables|SetLocalDelta (Math|Vector|MakeVector (.X (Math|Vector|BreakVector (- (Variables|Default|GetStartSwipeCoords%20	) (LocalVariables|GetLocalNewSwipeCoords)))) (.Y (Math|Vector|BreakVector (- (Variables|Default|GetStartSwipeCoords%20	) (LocalVariables|GetLocalNewSwipeCoords)))) 0.0)))
  (return _output_get))

(fn IsScrolling
  (bind (_sizex _sizey) (HUD|GetViewportSize))
  (bind (_locationx _locationy) (Game|Player|GetMousePosition))
  (bind _returnvalue (Math|Conversions|ToFloat(Integer) _sizex))
  (bind _returnvalue_2 (* _returnvalue 0.1))
  (bind _returnvalue_3 (< _locationx _returnvalue_2))
  (Utilities|FlowControl|Sequence
    (:then_0
      (if _returnvalue_3
        (LocalVariables|SetLocal%20Draq "CenterLeft")))
    (:then_1
      (if (and (not _returnvalue_3) (> (.LocationX (Game|Player|GetMousePosition)) (* (Math|Conversions|ToFloat(Integer) (.SizeX (HUD|GetViewportSize))) 0.9)))
        (LocalVariables|SetLocal%20Draq "CenterRight")))
    (:then_2
      (if true
        (LocalVariables|SetLocal%20Draq "MouseDown")))
    (:then_3
      (if true
        (LocalVariables|SetLocal%20Draq "MouseDown")))
    (:then_4
      (if true
        (LocalVariables|SetLocal%20Draq "MouseDown")))
    (:then_5
      (if true
        _))))